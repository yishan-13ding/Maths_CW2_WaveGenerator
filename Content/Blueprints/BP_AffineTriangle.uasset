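; BP_AffineTriangle is an actor Blueprint that computes affine-transformed vertex positions, by its name for a triangle.
; CalculateTransformedVertices builds a transform from the current translation, rotation and uniform scale, applies it to each input vertex, and returns the collected results.
; The event graph and construction script are empty, so nothing in this Blueprint calls the function or draws the result.
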(fn `CalculateTransformedVertices`
  (params (InVertices :type "Array of Vector Structure"))
  (returns (OutVertices :type "Array of Vector Structure"))
  (locals (TempVertices :type "Vector Structure"))
  (bind _currentscale (`self.CurrentScale`))
  (for _array_element InVertices
    (`KismetArrayLibrary.Array_Add` (`|MakeArray` (`KismetMathLibrary.TransformLocation` (`KismetMathLibrary.MakeTransform` (`self.CurrentTranslation`) (`self.CurrentRotation`) (`KismetMathLibrary.MakeVector` _currentscale _currentscale _currentscale)) _array_element)) (`local.TempVertices`)))
  (return (`|MakeArray` (`local.TempVertices`))))

(fn `UserConstructionScript`)